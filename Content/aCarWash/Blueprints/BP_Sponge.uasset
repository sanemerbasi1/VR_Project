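; BP_Sponge is a car wash sponge that paints onto BP_Target actors it touches, apparently to clean them.
; Box overlap events flag contact with a target.
; While flagged, Tick runs a one-unit multi box trace along the box's up vector, with debug drawing enabled.
; Each target hit gets a DrawToRenderTarget call at the impact point, sized from the box extent, with RainClean switched on only for that call.
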(event `self.Box.OnComponentBeginOverlap`
  (params (OverlappedComponent :type "PrimitiveComponent Object Reference") (OtherActor :type "Actor Object Reference") (OtherComp :type "PrimitiveComponent Object Reference") (OtherBodyIndex :type Integer) (bFromSweep :type Boolean) (SweepResult :type "HitResult Structure (by ref)"))
  (bind _asbp_target (cast `/Game/aCarWash/Blueprints/BP_Target` OtherActor))
  (bind _output_get (set `self.As BP Target` _asbp_target))
  (`/Engine/EditorBlueprintResources/StandardMacros.IsValid` _output_get
    (:`Is Valid`
      (set `self.IsOverlapping` true))))

(event `self.Box.OnComponentEndOverlap`
  (params (OverlappedComponent :type "PrimitiveComponent Object Reference") (OtherActor :type "Actor Object Reference") (OtherComp :type "PrimitiveComponent Object Reference") (OtherBodyIndex :type Integer))
  (bind _asbp_target (cast `/Game/aCarWash/Blueprints/BP_Target` OtherActor))
  (`/Engine/EditorBlueprintResources/StandardMacros.IsValid` _asbp_target
    (:`Is Valid`
      (set `self.IsOverlapping` false))))

(event `self.ReceiveTick`
  (params (DeltaSeconds :type "Float (single-precision)"))
  (bind _returnvalue (`SceneComponent.K2_GetComponentLocation` (`self.Box`)))
  (bind (_boxextent_x _boxextent_y _boxextent_z) (`KismetMathLibrary.BreakVector` (`BoxComponent.BoxExtent` (`self.Box`))))
  ; bitmedi
  (if (`self.IsOverlapping`)
    (bind _outhits (`KismetSystemLibrary.BoxTraceMulti` :`Start` _returnvalue :`End` (+ (`SceneComponent.GetUpVector` (`self.Box`)) _returnvalue) :`HalfSize` (`BoxComponent.GetScaledBoxExtent` (`self.Box`)) :`Orientation` (`SceneComponent.K2_GetComponentRotation` (`self.DefaultSceneRoot`)) :`TraceChannel` "TraceTypeQuery1" :`DrawDebugType` "ForOneFrame"))
    (for _array_element _outhits
      (bind (_bblockinghit _binitialoverlap _time _distance _location _impactpoint _normal _impactnormal _physmat _hitactor) (`GameplayStatics.BreakHitResult` _array_element))
      (bind _asbp_target (cast `/Game/aCarWash/Blueprints/BP_Target` _hitactor))
      (set `/Game/aCarWash/Blueprints/BP_Target.RainClean` true _asbp_target)
      (`/Game/aCarWash/Blueprints/BP_Target.DrawToRenderTarget` _asbp_target _impactpoint 10.0 (`KismetMathLibrary.MakeVector` (* _boxextent_x 0.6) _boxextent_y (* _boxextent_z 0.05)))
      (set `/Game/aCarWash/Blueprints/BP_Target.RainClean` false _asbp_target))))

(fn `UserConstructionScript`)