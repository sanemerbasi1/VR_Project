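; Grabbable VR water hose for the car wash that sprays water and cleans foam and dirt off targets.
; Grabbing enables input, adds a hand-specific Enhanced Input mapping context and hides that hand's message without casting to the pawn.
; Spraying moves a pre-spawned Niagara system to the nozzle and line traces forward.
; On a BP_Targett hit near foam, it paints the target's render target and destroys that foam component.
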(event OnGrabbed(GrabComponentSnap)
  (bind _grabcomponentsnap (Variables|Default|GetGrabComponentSnap))
  (bind _returnvalue (Default|GetHeldbyHand _grabcomponentsnap))
  (bind _returnvalue_2 (Utilities|Enum|Equal(Enum) _returnvalue "Right"))
  (Variables|Default|SetIsGrabbed true)
  (Input|EnableInput (Game|GetPlayerController 0))
  (Class|BPIPawnAnim|HideUnhideHand(Message) (Components|GetOwner (Variables|/Game/VRTemplate/Blueprints/GrabComponent.GrabComponent_C|GetMotionControllerRef _grabcomponentsnap)) true _returnvalue_2)
  (Input|AddMappingContext (PlayerController|LocalPlayerSubsystems|GetEnhancedInputLocalPlayerSubsystem (Game|GetPlayerController 0)) (select _returnvalue_2 "/Game/VRTemplate/Input/IMC_Weapon_Right.IMC_Weapon_Right" "/Game/VRTemplate/Input/IMC_Weapon_Left.IMC_Weapon_Left") 1 "(bIgnoreAllPressedKeysUntilRelease=True,bForceImmediately=False,bNotifyUserSettings=False)"))

(event OnDropped(GrabComponentSnap)
  (bind _grabcomponentsnap (Variables|Default|GetGrabComponentSnap))
  (bind _returnvalue (Default|GetHeldbyHand _grabcomponentsnap))
  (bind _returnvalue_2 (Utilities|Enum|Equal(Enum) _returnvalue "Right"))
  (Variables|Default|SetIsGrabbed false)
  (Components|Activation|Deactivate (Variables|Default|GetNiagaraWaterSystem))
  (Audio|Components|Audio|FadeOut (Variables|Default|GetAudio) 1.0 0.0 "Linear" :!class /Script/Engine.AudioComponent)
  (Input|DisableInput (Game|GetPlayerController 0))
  (Class|BPIPawnAnim|HideUnhideHand(Message) (Components|GetOwner (Variables|/Game/VRTemplate/Blueprints/GrabComponent.GrabComponent_C|GetMotionControllerRef _grabcomponentsnap)) false _returnvalue_2)
  (Input|RemoveMappingContext (PlayerController|LocalPlayerSubsystems|GetEnhancedInputLocalPlayerSubsystem (Game|GetPlayerController 0)) (select _returnvalue_2 "/Game/VRTemplate/Input/IMC_Weapon_Right.IMC_Weapon_Right" "/Game/VRTemplate/Input/IMC_Weapon_Left.IMC_Weapon_Left") "(bIgnoreAllPressedKeysUntilRelease=True,bForceImmediately=False,bNotifyUserSettings=False)"))

(event Custom|Spray
  (bind _muzzlelocation (Variables|Default|GetMuzzleLocation))
  (bind _watergun (Variables|Default|GetWaterGun))
  (bind _niagarawatersystem (Variables|Default|GetNiagaraWaterSystem))
  (bind _returnvalue (Transformation|GetWorldLocation _muzzlelocation))
  (Transformation|SetWorldLocationAndRotation _niagarawatersystem (Transformation|GetWorldLocation _watergun) (Transformation|GetWorldRotation _watergun) false false)
  (Components|Activation|Activate _niagarawatersystem false)
  (bind _outhit (Collision|LineTraceByChannel _returnvalue (+ (* (Math|Vector|GetForwardVector (Variables|Default|GetMuzzleLocation)) 3e+02) _returnvalue) "TraceTypeQuery1" false 0 "ForOneFrame"))
  (bind _asbp_targett (Utilities|Casting|CastToBP_Targett (.HitActor (Collision|BreakHitResult _outhit))))
  (Variables|Default|SetAs%20BP%20Target%20Test _asbp_targett)
  (for _array_element (Variables|/Game/aCarWash/Blueprints/BP_Targett.BP_Targett_C|GetFoamFX (Variables|Default|GetAs%20BP%20Target%20Test))
    (Utilities|IsValid _array_element
      (:Is%20Valid
        (if (Utilities|Operators|EqualEqual (Transformation|GetWorldLocation _array_element) (.ImpactPoint (Collision|BreakHitResult _outhit)) 15.0)
          (Default|DrawtoRenderTarget (Variables|Default|GetAs%20BP%20Target%20Test) (.ImpactPoint (Collision|BreakHitResult _outhit)) 3e+01 "0, 0, 0" "/Game/aCarWash/Material/M_RedBrush.M_RedBrush" "NewEnumerator0")
          (if (< (Math|Vector|Distance(Vector) (Transformation|GetWorldLocation _array_element) (.Location (Collision|BreakHitResult _outhit))) 15.0)
            (Components|DestroyComponent _array_element)))))))

(event Input|EnhancedActionEvents|EnhancedInputActionIA_Shoot_Left
  (params (ActionValue :type Boolean) (ElapsedSeconds :type Float%20%28double-precision%29) (TriggeredSeconds :type Float%20%28double-precision%29) (InputAction :type Input%20Action%20Object%20Reference :default "/Game/VRTemplate/Input/Actions/IA_Shoot_Left.IA_Shoot_Left"))
  (:Triggered
    (CallFunction|Spray :!label _label))
  (:Started
    (goto _label)))

(event Input|EnhancedActionEvents|EnhancedInputActionIA_Shoot_Right
  (params (ActionValue :type Boolean) (ElapsedSeconds :type Float%20%28double-precision%29) (TriggeredSeconds :type Float%20%28double-precision%29) (InputAction :type Input%20Action%20Object%20Reference :default "/Game/VRTemplate/Input/Actions/IA_Shoot_Right.IA_Shoot_Right"))
  (:Triggered
    (if (Variables|Default|GetIsGrabbed)
      (CallFunction|Spray)))
  (:Started
    (if (Variables|Default|GetIsGrabbed)
      (Audio|Components|Audio|Play (Variables|Default|GetAudio) 0.0)
      (else
        (Components|Activation|Deactivate (Variables|Default|GetNiagaraWaterSystem) :!label _label)
        (Audio|Components|Audio|FadeOut (Variables|Default|GetAudio) 1.0 0.0 "Linear" :!class /Script/Engine.AudioComponent))))
  (:Canceled
    (goto _label))
  (:Completed
    (goto _label)))

(event EventBeginPlay
  (bind _watergun (Variables|Default|GetWaterGun))
  (bind _asvrpawn (Utilities|Casting|CastToVRPawn (Game|Player|GetPlayerPawn 0)))
  (Variables|Default|SetAs%20VRPawn _asvrpawn)
  (bind _returnvalue (Niagara|SpawnSystematLocation "/Game/aCarWash/Other/FX_WaterGun.FX_WaterGun" (Transformation|GetWorldLocation _watergun) (Transformation|GetWorldRotation _watergun) "1.000000,1.000000,1.000000" false false))
  (Variables|Default|SetNiagaraWaterSystem _returnvalue))

(event EventTick
  (params (DeltaSeconds :type Float%20%28single-precision%29)))

(event Input|KeyboardEvents|DebugKeyE
  (params (Key :type Key%20Structure :default "None") (ActionValue :type Input%20Action%20Value%20Structure))
  (:Pressed
    (CallFunction|Spray))
  (:Released
    (Components|Activation|Deactivate (Variables|Default|GetNiagaraWaterSystem))
    (Audio|Components|Audio|FadeOut (Variables|Default|GetAudio) 1.0 0.0 "Linear" :!class /Script/Engine.AudioComponent)))

(fn ConstructionScript)