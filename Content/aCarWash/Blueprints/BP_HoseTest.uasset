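; BP_HoseTest is a test VR hose that paints onto BP_TargetTest actors where it points.
; GrabComponentSnap toggles input, the per-hand weapon mapping context and the pawn's hand message on grab and drop.
; Spray runs from shoot inputs and every Tick, even ungrabbed, line tracing briefly from the muzzle with debug drawing and calling DrawToRenderTarget at the impact.
; Water FX and foam removal logic is disconnected.
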(event `EnhancedInput|/Game/VRTemplate/Input/Actions/IA_Shoot_Left`
  (params (ActionValue :type Boolean) (ElapsedSeconds :type "Float (double-precision)") (TriggeredSeconds :type "Float (double-precision)") (InputAction :type "InputAction Object Reference" :default "/Game/VRTemplate/Input/Actions/IA_Shoot_Left.IA_Shoot_Left"))
  (:`Triggered`
    (`self.Spray` :!label _label))
  (:`Started`
    (goto _label)))

(event `self.ReceiveTick`
  (params (DeltaSeconds :type "Float (single-precision)"))
  (`self.Spray` :!label _label_2))

(event `EnhancedInput|/Game/VRTemplate/Input/Actions/IA_Shoot_Right`
  (params (ActionValue :type Boolean) (ElapsedSeconds :type "Float (double-precision)") (TriggeredSeconds :type "Float (double-precision)") (InputAction :type "InputAction Object Reference" :default "/Game/VRTemplate/Input/Actions/IA_Shoot_Right.IA_Shoot_Right"))
  (:`Triggered`
    (goto _label_2))
  (:`Started`
    (goto _label_2)))

(event `self.GrabComponentSnap.OnGrabbed`
  (bind _grabcomponentsnap (`self.GrabComponentSnap`))
  (bind _returnvalue (`|EnumEquality` (`/Game/VRTemplate/Blueprints/GrabComponent.GetHeldByHand` _grabcomponentsnap) "Right"))
  (set `self.IsGrabbed` true)
  (`self.EnableInput` (`GameplayStatics.GetPlayerController` 0))
  (message `/Game/VRTemplate/Blueprints/BPI_PawnAnim.HideUnhideHand` (`ActorComponent.GetOwner` (`/Game/VRTemplate/Blueprints/GrabComponent.MotionControllerRef` _grabcomponentsnap)) true _returnvalue)
  (`EnhancedInputSubsystemInterface.AddMappingContext` (pcsubsystem `EnhancedInputLocalPlayerSubsystem` (`GameplayStatics.GetPlayerController` 0)) (select `bool` _returnvalue :`false` "/Game/VRTemplate/Input/IMC_Weapon_Left.IMC_Weapon_Left" :`true` "/Game/VRTemplate/Input/IMC_Weapon_Right.IMC_Weapon_Right" :!type "InputMappingContext Object Reference") 1 (struct)))

(event `self.GrabComponentSnap.OnDropped`
  (bind _grabcomponentsnap (`self.GrabComponentSnap`))
  (bind _returnvalue (`|EnumEquality` (`/Game/VRTemplate/Blueprints/GrabComponent.GetHeldByHand` _grabcomponentsnap) "Right"))
  (set `self.IsGrabbed` false)
  (`self.DisableInput` (`GameplayStatics.GetPlayerController` 0))
  (message `/Game/VRTemplate/Blueprints/BPI_PawnAnim.HideUnhideHand` (`ActorComponent.GetOwner` (`/Game/VRTemplate/Blueprints/GrabComponent.MotionControllerRef` _grabcomponentsnap)) false _returnvalue)
  (`EnhancedInputSubsystemInterface.RemoveMappingContext` (pcsubsystem `EnhancedInputLocalPlayerSubsystem` (`GameplayStatics.GetPlayerController` 0)) (select `bool` _returnvalue :`false` "/Game/VRTemplate/Input/IMC_Weapon_Left.IMC_Weapon_Left" :`true` "/Game/VRTemplate/Input/IMC_Weapon_Right.IMC_Weapon_Right" :!type "InputMappingContext Object Reference") (struct)))

(event `self.ReceiveBeginPlay`
  (bind _asvrpawn (cast `/Game/VRTemplate/Blueprints/VRPawn` (`GameplayStatics.GetPlayerPawn` 0)))
  (set `self.As VRPawn` _asvrpawn))

(event `Spray`
  (bind _returnvalue (`SceneComponent.K2_GetComponentLocation` (`self.MuzzleLocation`)))
  (bind _outhit (`KismetSystemLibrary.LineTraceSingle` :`Start` _returnvalue :`End` (+ (* (`SceneComponent.GetForwardVector` (`self.MuzzleLocation`)) 100.0) _returnvalue) :`TraceChannel` "TraceTypeQuery1" :`DrawDebugType` "ForOneFrame"))
  (bind (_bblockinghit _binitialoverlap _time _distance _location _impactpoint _normal _impactnormal _physmat _hitactor) (`GameplayStatics.BreakHitResult` _outhit))
  (bind _asbp_target_test (cast `/Game/aCarWash/Blueprints/BP_TargetTest` _hitactor))
  (`/Game/aCarWash/Blueprints/BP_TargetTest.DrawToRenderTarget` _asbp_target_test _impactpoint 10.0 (0.0 0.0 0.0)))

(fn `UserConstructionScript`)