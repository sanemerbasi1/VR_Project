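; Car wash target actor that shows any assigned mesh with dirt and glass materials and lets brushes paint onto it.
; On BeginPlay it creates dynamic materials, briefly swaps in an unwrap material to capture a UV position render target, and binds a hit-mask target to the materials.
; DrawToRenderTarget stamps circular or square squeegee brushes into that mask at impact points, optionally setting spray color.
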(event `self.ReceiveBeginPlay`
  (bind _rt_hit (`self.RT Hit`))
  ; Except the glass material, for loop for all the materials in car to make them dynamic dirt material
  (for _index (range (`PrimitiveComponent.GetNumMaterials` (`self.CarMesh`)))
    (if (!= _index 1)
      (bind _returnvalue (`PrimitiveComponent.CreateDynamicMaterialInstance` (`self.CarMesh`) _index (`self.SourceMaterial`) "None"))
      (set `self.DirtDynamicMaterial` _returnvalue)
      (`KismetArrayLibrary.Array_Add` (`self.Material Instances`) _returnvalue)
      (else
        (bind _returnvalue_2 (`PrimitiveComponent.CreateDynamicMaterialInstance` (`self.CarMesh`) 0 "/Game/aCarWash/Other/M_MasterGlass_Inst.M_MasterGlass_Inst" "None"))
        (set `self.GlassDynamicMaterial` _returnvalue_2)
        (`KismetArrayLibrary.Array_Add` (`self.Material Instances`) _returnvalue_2))))
  (`|ExecutionSequence`
    (:`then_0`
      ; Set values of the material and get UV Render
      (bind _returnvalue_3 (`KismetRenderingLibrary.CreateRenderTarget2D` 1024 1024))
      (bind _output_get (set `self.RT Unwrap` _returnvalue_3))
      (set `SceneCaptureComponent2D.TextureTarget` _output_get (`self.SceneCaptureComponent2D`))
      (`SceneCaptureComponent.ShowOnlyActorComponents` (`self.SceneCaptureComponent2D`) self false))
    (:`then_1`
      (bind _returnvalue_4 (`KismetRenderingLibrary.CreateRenderTarget2D` 1024 1024))
      (set `self.RT Hit` _returnvalue_4)
      (for _array_element (`self.Material Instances`)
        (`MaterialInstanceDynamic.SetTextureParameterValueByInfo` _array_element (make `MaterialParameterInfo` "OpacityMask" "BlendParameter" 0) _rt_hit)
        (`MaterialInstanceDynamic.SetTextureParameterValue` _array_element "RT_Hit" _rt_hit)))
    (:`then_2`
      (`SceneComponent.K2_SetWorldRotation` (`self.SceneCaptureComponent2D`) (struct :`Pitch` -90.0 :`Yaw` -90.0) false false)
      (for _index_2 (range (`PrimitiveComponent.GetNumMaterials` (`self.CarMesh`)))
        (`PrimitiveComponent.SetMaterial` (`self.CarMesh`) _index_2 "/Game/aCarWash/Other/M_Unwrap.M_Unwrap"))
      (`SceneCaptureComponent2D.CaptureScene` (`self.SceneCaptureComponent2D`))
      (for (_array_element_2 _array_index) (`self.Material Instances`)
        (`PrimitiveComponent.SetMaterial` (`self.CarMesh`) _array_index _array_element_2))
      (bind _returnvalue_5 (`KismetMaterialLibrary.CreateDynamicMaterialInstance` "/Game/aCarWash/Other/M_BrushSquare.M_BrushSquare"))
      (bind _output_get_2 (set `self.ML BrushSquare` _returnvalue_5))
      (`MaterialInstanceDynamic.SetTextureParameterValue` _output_get_2 "UnwrappedSquare" (`self.RT Unwrap`)))))

(fn `DrawToRenderTarget`
  (params (`Impact Point` :type "Vector Structure") (BrushSize :type "Float (double-precision)") (BoxExtend :type "Vector Structure") (BrushMaterial :type "Material Object Reference") (Enum :type "/Game/aCarWash/Material/Enum_Brushes Enum" :default "NewEnumerator0") (`Color Value` :type "LinearColor Structure"))
  (bind _returnvalue (`KismetMaterialLibrary.CreateDynamicMaterialInstance` BrushMaterial))
  (if (`|EnumEquality` Enum "NewEnumerator1")
    (for _array_element (`self.Material Instances`)
      (`MaterialInstanceDynamic.SetVectorParameterValue` _array_element "SprayColor" `Color Value`))
    ; Set parameters and then Draw to Render Target Circular
    (`MaterialInstanceDynamic.SetTextureParameterValue` _returnvalue "Unwrapped" (`self.RT Unwrap`) :!label _label)
    (set `self.MI Brush` _returnvalue)
    (`MaterialInstanceDynamic.SetScalarParameterValue` (`self.MI Brush`) "Size" BrushSize)
    (`MaterialInstanceDynamic.SetVectorParameterValue` (`self.MI Brush`) "Position" (`KismetMathLibrary.Conv_VectorToLinearColor` (`local.Impact Point`)))
    (`MaterialInstanceDynamic.SetTextureParameterValue` (`self.MI Brush`) "RT_Hit" (`self.RT Hit`))
    (`KismetRenderingLibrary.DrawMaterialToRenderTarget` (`self.RT Hit`) (`self.MI Brush`))
    (else
      ; Square Brush for Squeege
      (if (== BrushMaterial "/Game/aCarWash/Material/M_BlueBrushSquare.M_BlueBrushSquare")
        (`MaterialInstanceDynamic.SetTextureParameterValue` _returnvalue "Unwrapped" (`self.RT Unwrap`))
        (set `self.MI Brush` _returnvalue)
        (`MaterialInstanceDynamic.SetVectorParameterValue` (`self.MI Brush`) "Size" (`KismetMathLibrary.Conv_VectorToLinearColor` BoxExtend))
        (`MaterialInstanceDynamic.SetVectorParameterValue` (`self.MI Brush`) "Position" (`KismetMathLibrary.Conv_VectorToLinearColor` (`local.Impact Point`)))
        (`MaterialInstanceDynamic.SetTextureParameterValue` (`self.MI Brush`) "RT_Hit" (`self.RT Hit`))
        (`KismetRenderingLibrary.DrawMaterialToRenderTarget` (`self.RT Hit`) (`self.MI Brush`))
        (else
          (goto _label))))))

(fn `ModifyBrushSize`
  (params (BrushSize :type "Float (double-precision)" :default 0.0))
  ; Set the size parameter
  (`MaterialInstanceDynamic.SetScalarParameterValue` (`self.MI Brush`) "Size" BrushSize))

(fn `UserConstructionScript`
  ; Put any mesh you want to the target blueprint
  (`StaticMeshComponent.SetStaticMesh` (`self.CarMesh`) (`self.SourceMesh`))
  (`PrimitiveComponent.SetMaterial` (`self.CarMesh`) 1 (`self.SourceMaterial`)))