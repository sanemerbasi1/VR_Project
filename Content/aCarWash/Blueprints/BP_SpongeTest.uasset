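; BP_SpongeTest is a test sponge actor for the car wash that paints onto BP_Targett surfaces while touching them.
; A Box overlap with a BP_Targett sets or clears an overlap flag.
; While that flag is set, Tick fires a short Visibility line trace along the LineTrace component's up vector.
; A hit on a BP_Targett calls its DrawToRenderTarget at the impact point with a blue brush material.
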(event `self.Box.OnComponentBeginOverlap`
  (params (OverlappedComponent :type "PrimitiveComponent Object Reference") (OtherActor :type "Actor Object Reference") (OtherComp :type "PrimitiveComponent Object Reference") (OtherBodyIndex :type Integer) (bFromSweep :type Boolean) (SweepResult :type "HitResult Structure (by ref)"))
  (bind _asbp_targett (cast `/Game/aCarWash/Blueprints/BP_Targett` OtherActor))
  (`/Engine/EditorBlueprintResources/StandardMacros.IsValid` _asbp_targett
    (:`Is Valid`
      (set `self.IsOverlapping` true)
      (`KismetSystemLibrary.PrintString` "Hello"))))

(event `self.Box.OnComponentEndOverlap`
  (params (OverlappedComponent :type "PrimitiveComponent Object Reference") (OtherActor :type "Actor Object Reference") (OtherComp :type "PrimitiveComponent Object Reference") (OtherBodyIndex :type Integer))
  (bind _asbp_targett (cast `/Game/aCarWash/Blueprints/BP_Targett` OtherActor))
  (`/Engine/EditorBlueprintResources/StandardMacros.IsValid` _asbp_targett
    (:`Is Valid`
      (set `self.IsOverlapping` false))))

(event `self.ReceiveTick`
  (params (DeltaSeconds :type "Float (single-precision)"))
  (bind _linetrace (`self.LineTrace`))
  (bind _returnvalue (`SceneComponent.K2_GetComponentLocation` _linetrace))
  ; bitmedi
  (if (`self.IsOverlapping`)
    (bind (_outhit _returnvalue_2) (`KismetSystemLibrary.LineTraceSingle` :`Start` _returnvalue :`End` (+ (* (`SceneComponent.GetUpVector` _linetrace) 10.0) _returnvalue) :`TraceChannel` "TraceTypeQuery1" :`DrawDebugType` "ForOneFrame"))
    (if _returnvalue_2
      (bind (_bblockinghit _binitialoverlap _time _distance _location _impactpoint _normal _impactnormal _physmat _hitactor) (`GameplayStatics.BreakHitResult` _outhit))
      (bind _asbp_targett (cast `/Game/aCarWash/Blueprints/BP_Targett` _hitactor))
      (`/Game/aCarWash/Blueprints/BP_Targett.DrawToRenderTarget` :`self` _asbp_targett :`Impact Point` _impactpoint :`BrushSize` 20.0 :`BoxExtend` (0.0 0.0 0.0) :`BrushMaterial` "/Game/aCarWash/Material/M_BlueBrush.M_BlueBrush"))))

(fn `UserConstructionScript`)