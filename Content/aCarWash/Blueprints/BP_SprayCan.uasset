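; BP_SprayCan is a grabbable spray can actor in the car wash game that works alongside a spray gun Blueprint.
; On BeginPlay it creates a dynamic material instance on its cylinder mesh and tints it with the can's color.
; GrabComponentSnap events track whether it is held, and grabbing it hides the spray gun's child can visual if the gun's IsAttached flag is set.
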(event `self.ReceiveBeginPlay`
  (bind _cylinder (`self.Cylinder`))
  (bind _returnvalue (`PrimitiveComponent.CreateDynamicMaterialInstance` _cylinder 0 (`PrimitiveComponent.GetMaterial` _cylinder 0) "None"))
  (set `self.CanMatDMI` _returnvalue)
  (`MaterialInstanceDynamic.SetVectorParameterValue` _returnvalue "CanBaseColor" (`self.CanColor`)))

(event `self.GrabComponentSnap.OnGrabbed`
  (bind _bp_spraygun (`self.BP_SprayGun`))
  (set `self.IsGrabbed` true)
  (if (`/Game/aCarWash/Blueprints/BP_SprayGun.IsAttached` _bp_spraygun)
    (`SceneComponent.SetVisibility` (`/Game/aCarWash/Blueprints/BP_SprayGun.SprayCanChild` _bp_spraygun) false false)))

(event `self.GrabComponentSnap.OnDropped`
  (set `self.IsGrabbed` false))

(fn `UserConstructionScript`)