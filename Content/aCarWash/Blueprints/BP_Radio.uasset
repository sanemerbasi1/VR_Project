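; BP_Radio is a car wash radio that the VR player triggers by touch to cycle through music tracks.
; The A input enables collision on the VRPawn's sphere for half a second, letting it overlap the radio's sphere.
; The first overlap only sets IsOpen; later ones play the next of three sounds and spin a scene component one full pitch turn via a timeline.
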(event `EnhancedInput|/Game/VRTemplate/Input/Actions/IA_A`
  (params (ActionValue :type Boolean) (ElapsedSeconds :type "Float (double-precision)") (TriggeredSeconds :type "Float (double-precision)") (InputAction :type "InputAction Object Reference" :default "/Game/VRTemplate/Input/Actions/IA_A.IA_A"))
  (:`Triggered`
    (bind _asvrpawn (cast `/Game/VRTemplate/Blueprints/VRPawn` (`GameplayStatics.GetPlayerPawn` 0)))
    (`PrimitiveComponent.SetCollisionEnabled` (`/Game/VRTemplate/Blueprints/VRPawn.Sphere` _asvrpawn) "QueryAndPhysics")
    (`KismetSystemLibrary.Delay` 0.5)
    (bind _asvrpawn_2 (cast `/Game/VRTemplate/Blueprints/VRPawn` (`GameplayStatics.GetPlayerPawn` 0)))
    (`PrimitiveComponent.SetCollisionEnabled` (`/Game/VRTemplate/Blueprints/VRPawn.Sphere` _asvrpawn_2) "NoCollision")))

(event `self.Sphere.OnComponentBeginOverlap`
  (params (OverlappedComponent :type "PrimitiveComponent Object Reference") (OtherActor :type "Actor Object Reference") (OtherComp :type "PrimitiveComponent Object Reference") (OtherBodyIndex :type Integer) (bFromSweep :type Boolean) (SweepResult :type "HitResult Structure (by ref)"))
  (bind _radio_music (`self.radio_music`))
  (if (== (`GameplayStatics.GetPlayerPawn` 0) OtherActor)
    (bind _asvrpawn (cast `/Game/VRTemplate/Blueprints/VRPawn` OtherActor))
    (`KismetSystemLibrary.PrintString` "Hello")
    (`/Engine/EditorBlueprintResources/StandardMacros.IsValid` _asvrpawn
      (:`Is Valid`
        (if (`self.IsOpen`)
          (bind _output_get (set `self.CurrentIndex` (mod (+ (`self.CurrentIndex`) 1) 3)))
          (`AudioComponent.SetSound` _radio_music (`|GetArrayItem` (`self.SoundArray`) _output_get))
          (`AudioComponent.Play` _radio_music 0.0)
          (bind (_direction _buttonround) (`Timeline|ButtonTimeline` :!via `PlayFromStart`)
            (:`Update`
              (`SceneComponent.K2_SetWorldRotation` (`self.Scene`) (`KismetMathLibrary.MakeRotator` 0.0 (`KismetMathLibrary.Lerp` 0.0 -360.0 _buttonround)) false false)))
          (else
            (set `self.IsOpen` true)))))))

(fn `UserConstructionScript`)