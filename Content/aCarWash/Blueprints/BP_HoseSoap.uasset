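; BP_HoseSoap is a grabbable VR foam gun that sprays soap onto BP_Targett actors in the car wash.
; Grabbing enables input, adds the hand's weapon mapping context and hides that hand's message on the controller's owner; dropping reverses this.
; Shoot inputs and a debug R key call Spray, with looping-style audio control only on right-hand and debug paths.
; Spray spawns muzzle foam, line-traces forward, and adds impact foam to the target's FoamFX array.
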(event OnGrabbed(GrabComponent)
  (bind _grabcomponent (Variables|Default|GetGrabComponent))
  (bind _returnvalue (Default|GetHeldbyHand _grabcomponent))
  (bind _returnvalue_2 (Utilities|Enum|Equal(Enum) _returnvalue "Right"))
  (Variables|Default|SetIsGrabbed true)
  (Input|EnableInput (Game|GetPlayerController 0))
  (Class|BPIPawnAnim|HideUnhideHand(Message) (Components|GetOwner (Variables|/Game/VRTemplate/Blueprints/GrabComponent.GrabComponent_C|GetMotionControllerRef _grabcomponent)) true _returnvalue_2)
  (Input|AddMappingContext (PlayerController|LocalPlayerSubsystems|GetEnhancedInputLocalPlayerSubsystem (Game|GetPlayerController 0)) (select _returnvalue_2 "/Game/VRTemplate/Input/IMC_Weapon_Right.IMC_Weapon_Right" "/Game/VRTemplate/Input/IMC_Weapon_Left.IMC_Weapon_Left") 1 "(bIgnoreAllPressedKeysUntilRelease=True,bForceImmediately=False,bNotifyUserSettings=False)"))

(event OnDropped(GrabComponent)
  (bind _grabcomponent (Variables|Default|GetGrabComponent))
  (bind _returnvalue (Default|GetHeldbyHand _grabcomponent))
  (bind _returnvalue_2 (Utilities|Enum|Equal(Enum) _returnvalue "Right"))
  (Variables|Default|SetIsGrabbed false)
  (Input|DisableInput (Game|GetPlayerController 0))
  (Audio|Components|Audio|FadeOut (Variables|Default|GetAudio) 1.0 0.0 "Linear" :!class /Script/Engine.AudioComponent)
  (Class|BPIPawnAnim|HideUnhideHand(Message) (Components|GetOwner (Variables|/Game/VRTemplate/Blueprints/GrabComponent.GrabComponent_C|GetMotionControllerRef _grabcomponent)) false _returnvalue_2)
  (Input|RemoveMappingContext (PlayerController|LocalPlayerSubsystems|GetEnhancedInputLocalPlayerSubsystem (Game|GetPlayerController 0)) (select _returnvalue_2 "/Game/VRTemplate/Input/IMC_Weapon_Right.IMC_Weapon_Right" "/Game/VRTemplate/Input/IMC_Weapon_Left.IMC_Weapon_Left") "(bIgnoreAllPressedKeysUntilRelease=True,bForceImmediately=False,bNotifyUserSettings=False)"))

(event Custom|Spray
  (bind _foamgun (Variables|Components|GetFoamGun))
  (bind _foamgun_2 (Variables|Components|GetFoamGun))
  (bind _muzzlelocation (Variables|Default|GetMuzzleLocation))
  (bind _returnvalue (Transformation|GetWorldLocation _muzzlelocation))
  (bind _returnvalue_2 (Niagara|SpawnSystematLocation "/Game/aCarWash/Other/FX_FoamGun.FX_FoamGun" (Transformation|GetWorldLocation _foamgun) (Transformation|GetWorldRotation _foamgun)))
  (Transformation|SetWorldLocationAndRotation _returnvalue_2 (Transformation|GetWorldLocation _foamgun_2) (Transformation|GetWorldRotation _foamgun_2) false false)
  (Components|Activation|Activate _returnvalue_2 false)
  (bind _outhit (Collision|LineTraceByChannel _returnvalue (+ (* (Math|Vector|GetForwardVector (Variables|Default|GetMuzzleLocation)) 3e+02) _returnvalue) "TraceTypeQuery1" false 0 "None"))
  (bind _asbp_targett (Utilities|Casting|CastToBP_Targett (.HitActor (Collision|BreakHitResult _outhit))))
  (Utilities|IsValid _asbp_targett
    (:Is%20Valid
      _)
    (:Is%20Not%20Valid
      _))
  (bind _returnvalue_3 (Niagara|SpawnSystematLocation "/Game/aCarWash/Other/FX_Foam_System.FX_Foam_System" (.Location (Collision|BreakHitResult _outhit))))
  (Utilities|Array|Add (Variables|/Game/aCarWash/Blueprints/BP_Targett.BP_Targett_C|GetFoamFX _asbp_targett) _returnvalue_3))

(event Input|EnhancedActionEvents|EnhancedInputActionIA_Shoot_Left
  (params (ActionValue :type Boolean) (ElapsedSeconds :type Float%20%28double-precision%29) (TriggeredSeconds :type Float%20%28double-precision%29) (InputAction :type Input%20Action%20Object%20Reference :default "/Game/VRTemplate/Input/Actions/IA_Shoot_Left.IA_Shoot_Left"))
  (:Triggered
    (CallFunction|Spray :!label _label))
  (:Started
    (goto _label)))

(event Input|EnhancedActionEvents|EnhancedInputActionIA_Shoot_Right
  (params (ActionValue :type Boolean) (ElapsedSeconds :type Float%20%28double-precision%29) (TriggeredSeconds :type Float%20%28double-precision%29) (InputAction :type Input%20Action%20Object%20Reference :default "/Game/VRTemplate/Input/Actions/IA_Shoot_Right.IA_Shoot_Right"))
  (:Triggered
    (if (Variables|Default|GetIsGrabbed)
      (CallFunction|Spray)))
  (:Started
    (if (Variables|Default|GetIsGrabbed)
      (Audio|Components|Audio|Play (Variables|Default|GetAudio) 0.0)))
  (:Canceled
    (Audio|Components|Audio|FadeOut (Variables|Default|GetAudio) 1.0 0.0 "Linear" :!class /Script/Engine.AudioComponent :!label _label))
  (:Completed
    (goto _label)))

(event EventBeginPlay
  (bind _asvrpawn (Utilities|Casting|CastToVRPawn (Game|Player|GetPlayerPawn 0)))
  (Variables|Default|SetAs%20VRPawn _asvrpawn))

(event Input|KeyboardEvents|DebugKeyR
  (params (Key :type Key%20Structure :default "None") (ActionValue :type Input%20Action%20Value%20Structure))
  (:Pressed
    (CallFunction|Spray))
  (:Released
    (Audio|Components|Audio|FadeOut (Variables|Default|GetAudio) 1.0 0.0 "Linear" :!class /Script/Engine.AudioComponent)))

(fn ConstructionScript)