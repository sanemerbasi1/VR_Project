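; Car wash cleaning actor that slides along world X on a timeline and attempts to erase dirt from surfaces it faces.
; Each Tick casts a 3x3 grid of short, debug-drawn forward traces.
; Each hit creates an M_CarDirt dynamic instance, sets its BrushCenter to the collision UV, then draws the separate M_CleaningMat asset into RT_CarDirt.
; The overlap event is empty; an older local-position brush approach is disconnected.
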(event `self.ReceiveTick`
  (params (DeltaSeconds :type "Float (single-precision)"))
  ; Line Tracing with 9x9 Grid
  (for _index (range 3)
    (for _index_2 (range 3)
      (bind _returnvalue (+ (`self.K2_GetActorLocation`) (* (* (- (/ (`KismetMathLibrary.Conv_IntToDouble` _index_2) 2.0) 0.5) 30.0) (`self.GetActorRightVector`)) (* (* (- (/ (`KismetMathLibrary.Conv_IntToDouble` _index) 2.0) 0.5) 20.0) (`self.GetActorUpVector`)) (* (`self.GetActorForwardVector`) 20.0)))
      (bind (_outhit _returnvalue_2) (`KismetSystemLibrary.LineTraceSingle` :`Start` _returnvalue :`End` (+ (* (`self.GetActorForwardVector`) 20.0) _returnvalue) :`TraceChannel` "TraceTypeQuery1" :`bTraceComplex` true :`DrawDebugType` "ForDuration"))
      (if _returnvalue_2
        (`KismetSystemLibrary.PrintString` "YESYESYESYESYESYES")
        (bind _returnvalue_3 (`PrimitiveComponent.CreateDynamicMaterialInstance` (`.HitComponent` (`GameplayStatics.BreakHitResult` _outhit)) 0 "/Game/aCarWash/Other/M_CarDirt.M_CarDirt" "None"))
        (set `self.CarMatInstance` _returnvalue_3)
        (bind _uv (`GameplayStatics.FindCollisionUV` _outhit))
        (`MaterialInstanceDynamic.SetVectorParameterValue` _returnvalue_3 "BrushCenter" (make `LinearColor` (`KismetMathLibrary.BreakVector2D` _uv) (`.Y` (`KismetMathLibrary.BreakVector2D` _uv)) 0.0 1.0))
        (`KismetRenderingLibrary.DrawMaterialToRenderTarget` "/Game/aCarWash/Other/RT_CarDirt.RT_CarDirt" "/Game/aCarWash/Other/M_CleaningMat.M_CleaningMat")
        (else
          (`KismetSystemLibrary.PrintString` "NONONONONONONO"))))))

(event `self.ReceiveBeginPlay`
  (bind (_returnvalue_x _returnvalue_y _returnvalue_z) (`KismetMathLibrary.BreakVector` (`self.K2_GetActorLocation`)))
  (bind (_direction _move) (`Timeline|Move`)
    (:`Update`
      (`self.K2_SetActorLocation` (`KismetMathLibrary.MakeVector` (`KismetMathLibrary.Lerp` -50.0 -100.0 _move) _returnvalue_y _returnvalue_z)))))

(event `self.Box.OnComponentBeginOverlap`
  (params (OverlappedComponent :type "PrimitiveComponent Object Reference") (OtherActor :type "Actor Object Reference") (OtherComp :type "PrimitiveComponent Object Reference") (OtherBodyIndex :type Integer) (bFromSweep :type Boolean) (SweepResult :type "HitResult Structure (by ref)")))

(fn `UserConstructionScript`)