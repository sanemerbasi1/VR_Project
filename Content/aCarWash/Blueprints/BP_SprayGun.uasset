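; VR grabbable spray gun that takes paint cans and sprays their color onto BP_Targett actors.
; Grabbing adds the hand's input mapping; overlapping a held BP_SprayCan hides it and tints the gun's can and Niagara spray.
; Shooting line-traces from the muzzle and paints the target's render target at the impact point.
; Player pawn overlap restores the can actor, though DeattachCan leaves IsAttached true.
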(event OnGrabbed(GrabComponentSnap)
  (bind _grabcomponentsnap (Variables|Default|GetGrabComponentSnap))
  (bind _returnvalue (Default|GetHeldbyHand _grabcomponentsnap))
  (bind _returnvalue_2 (Utilities|Enum|Equal(Enum) _returnvalue "Right"))
  (Variables|Default|SetIsGrabbed true)
  (Input|EnableInput (Game|GetPlayerController 0))
  (Class|BPIPawnAnim|HideUnhideHand(Message) (Components|GetOwner (Variables|/Game/VRTemplate/Blueprints/GrabComponent.GrabComponent_C|GetMotionControllerRef _grabcomponentsnap)) true _returnvalue_2)
  (Input|AddMappingContext (PlayerController|LocalPlayerSubsystems|GetEnhancedInputLocalPlayerSubsystem (Game|GetPlayerController 0)) (select _returnvalue_2 "/Game/VRTemplate/Input/IMC_Weapon_Right.IMC_Weapon_Right" "/Game/VRTemplate/Input/IMC_Weapon_Left.IMC_Weapon_Left") 1 "(bIgnoreAllPressedKeysUntilRelease=True,bForceImmediately=False,bNotifyUserSettings=False)"))

(event OnDropped(GrabComponentSnap)
  (bind _grabcomponentsnap (Variables|Default|GetGrabComponentSnap))
  (bind _returnvalue (Default|GetHeldbyHand _grabcomponentsnap))
  (bind _returnvalue_2 (Utilities|Enum|Equal(Enum) _returnvalue "Right"))
  (Variables|Default|SetIsGrabbed false)
  (Input|DisableInput (Game|GetPlayerController 0))
  (Audio|Components|Audio|FadeOut (Variables|Default|GetAudio) 1.0 0.0 "Linear" :!class /Script/Engine.AudioComponent)
  (Components|Activation|Deactivate (Variables|Default|GetNiagaraSpraySystem))
  (Class|BPIPawnAnim|HideUnhideHand(Message) (Components|GetOwner (Variables|/Game/VRTemplate/Blueprints/GrabComponent.GrabComponent_C|GetMotionControllerRef _grabcomponentsnap)) false _returnvalue_2)
  (Input|RemoveMappingContext (PlayerController|LocalPlayerSubsystems|GetEnhancedInputLocalPlayerSubsystem (Game|GetPlayerController 0)) (select _returnvalue_2 "/Game/VRTemplate/Input/IMC_Weapon_Right.IMC_Weapon_Right" "/Game/VRTemplate/Input/IMC_Weapon_Left.IMC_Weapon_Left") "(bIgnoreAllPressedKeysUntilRelease=True,bForceImmediately=False,bNotifyUserSettings=False)"))

(event OnComponentBeginOverlap(Sphere)
  (params (OverlappedComponent :type Primitive%20Component%20Object%20Reference) (OtherActor :type Actor%20Object%20Reference) (OtherComp :type Primitive%20Component%20Object%20Reference) (OtherBodyIndex :type Integer) (bFromSweep :type Boolean) (SweepResult :type Hit%20Result%20Structure%20%28by%20ref%29))
  (Utilities|FlowControl|Sequence
    (:then_0
      (bind _asbp_spray_can (Utilities|Casting|CastToBP_SprayCan OtherActor))
      (bind _output_get (Variables|Default|SetAs%20BP%20Spray%20Can _asbp_spray_can))
      (if (and (Variables|/Game/aCarWash/Blueprints/BP_SprayCan.BP_SprayCan_C|GetIsGrabbed _output_get) (not (Variables|Default|GetIsAttached)))
        (CallFunction|AttachCan)))
    (:then_1
      (if (== OtherActor (Game|Player|GetPlayerPawn 0))
        (if (Variables|Default|GetIsAttached)
          (CallFunction|DeattachCan))))))

(event Custom|Attach%20Can
  (Rendering|SetVisibility (Variables|Default|GetSprayCan) true false)
  (Rendering|Material|SetVectorParameterValueonMaterials (Variables|Default|GetSprayCan) "CanBaseColor" (Math|Conversions|ToVector(LinearColor) (Variables|/Game/aCarWash/Blueprints/BP_SprayCan.BP_SprayCan_C|GetCanColor (Variables|Default|GetAs%20BP%20Spray%20Can))))
  (Variables|Default|SetIsAttached true)
  (Niagara|SetNiagaraVariable(LinearColor) (Variables|Default|GetNiagaraSpraySystem) "User.SprayColor" (Variables|/Game/aCarWash/Blueprints/BP_SprayCan.BP_SprayCan_C|GetCanColor (Variables|Default|GetAs%20BP%20Spray%20Can)))
  (Development|PrintString "Attached")
  ;[0.15 0.15 0.15 0.5] Can'le işin bitince destroy
  (Rendering|SetActorHiddenInGame (Variables|Default|GetAs%20BP%20Spray%20Can) true))

(event Custom|Deattach%20Can
  (bind _as_bp_spray_can (Variables|Default|GetAs%20BP%20Spray%20Can))
  (Variables|Default|SetIsAttached true)
  (Development|PrintString "Deattached")
  (Rendering|SetActorHiddenInGame _as_bp_spray_can false)
  (Transformation|SetActorLocation _as_bp_spray_can (Transformation|GetWorldLocation (Variables|Default|GetSphere)) false true)
  (Rendering|SetVisibility (Variables|Default|GetSprayCan) false false))

(event Custom|Spray
  (bind _muzzlelocation (Variables|Default|GetMuzzleLocation))
  (bind _as_bp_spray_can (Variables|Default|GetAs%20BP%20Spray%20Can))
  (bind _niagaraspraysystem (Variables|Default|GetNiagaraSpraySystem))
  (bind _sprayfx (Variables|Default|GetSprayFX))
  (bind _returnvalue (Transformation|GetWorldLocation _muzzlelocation))
  (bind _canmatdmi (Variables|/Game/aCarWash/Blueprints/BP_SprayCan.BP_SprayCan_C|GetCanMatDMI _as_bp_spray_can))
  (Transformation|SetWorldLocationAndRotation _niagaraspraysystem (Transformation|GetWorldLocation _sprayfx) (Transformation|GetWorldRotation _sprayfx) false false)
  (Components|Activation|Activate _niagaraspraysystem false)
  (bind _outhit (Collision|LineTraceByChannel _returnvalue (+ (* (Math|Vector|GetForwardVector (Variables|Default|GetMuzzleLocation)) 3e+02) _returnvalue) "TraceTypeQuery1" false 0 "ForOneFrame"))
  (bind _asbp_targett (Utilities|Casting|CastToBP_Targett (.HitActor (Collision|BreakHitResult _outhit))))
  (bind _output_get (Variables|Default|SetAs%20BP%20Target%20Test _asbp_targett))
  (Rendering|Material|SetVectorParameterValue _canmatdmi "CanBaseColor" (Variables|/Game/aCarWash/Blueprints/BP_SprayCan.BP_SprayCan_C|GetCanColor (Variables|Default|GetAs%20BP%20Spray%20Can)) :!class /Script/Engine.MaterialInstanceDynamic)
  (bind _returnvalue_2 (Rendering|Material|GetVectorParameterValue _canmatdmi "CanBaseColor" :!class /Script/Engine.MaterialInstanceDynamic))
  (Default|DrawtoRenderTarget _output_get (.ImpactPoint (Collision|BreakHitResult _outhit)) 5.0 "0, 0, 0" "/Game/aCarWash/Material/M_GreenBrush.M_GreenBrush" "NewEnumerator1" _returnvalue_2))

(event Input|EnhancedActionEvents|EnhancedInputActionIA_Shoot_Left
  (params (ActionValue :type Boolean) (ElapsedSeconds :type Float%20%28double-precision%29) (TriggeredSeconds :type Float%20%28double-precision%29) (InputAction :type Input%20Action%20Object%20Reference :default "/Game/VRTemplate/Input/Actions/IA_Shoot_Left.IA_Shoot_Left"))
  (if (and (Variables|Default|GetIsGrabbed) (Variables|Default|GetIsAttached))
    (CallFunction|Spray)))

(event Input|EnhancedActionEvents|EnhancedInputActionIA_Shoot_Right
  (params (ActionValue :type Boolean) (ElapsedSeconds :type Float%20%28double-precision%29) (TriggeredSeconds :type Float%20%28double-precision%29) (InputAction :type Input%20Action%20Object%20Reference :default "/Game/VRTemplate/Input/Actions/IA_Shoot_Right.IA_Shoot_Right"))
  (:Triggered
    (if (and (Variables|Default|GetIsGrabbed) (Variables|Default|GetIsAttached))
      (CallFunction|Spray)))
  (:Started
    (if (and (Variables|Default|GetIsGrabbed) (Variables|Default|GetIsAttached))
      (Audio|Components|Audio|Play (Variables|Default|GetAudio) 0.0)))
  (:Canceled
    (Audio|Components|Audio|FadeOut (Variables|Default|GetAudio) 1.0 0.0 "Linear" :!class /Script/Engine.AudioComponent :!label _label)
    (Components|Activation|Deactivate (Variables|Default|GetNiagaraSpraySystem)))
  (:Completed
    (goto _label)))

(event EventBeginPlay
  (bind _sprayfx (Variables|Default|GetSprayFX))
  (bind _returnvalue (Niagara|SpawnSystematLocation "/Game/aCarWash/Other/FX_SprayCan.FX_SprayCan" (Transformation|GetWorldLocation _sprayfx) (Transformation|GetWorldRotation _sprayfx) "1.000000,1.000000,1.000000" false false))
  (Variables|Default|SetNiagaraSpraySystem _returnvalue))

(event Input|KeyboardEvents|DebugKeyE
  (params (Key :type Key%20Structure :default "None") (ActionValue :type Input%20Action%20Value%20Structure))
  (:Pressed
    (if (and (Variables|Default|GetIsGrabbed) (Variables|Default|GetIsAttached))
      (CallFunction|Spray))))

(fn ConstructionScript)